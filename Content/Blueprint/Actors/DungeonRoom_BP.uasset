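; DungeonRoom_BP is a room actor that builds a dungeon floor at runtime by spawning a grid of floor tile actors on BeginPlay.
; Nested loops over Yplanes and XPlane place tiles 100 units apart, centered on the world origin rather than the actor's location.
; Each tile rolls against ChangedMaxPerct to swap its Plane material for a random FloorMaterial entry, varying the floor's look.
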(event `self.ReceiveBeginPlay`
  (for _index (range (+ (`self.Yplanes`) 1))
    (for _index_2 (range (+ (`self.XPlane`) 1))
      (bind _returnvalue (`|SpawnActorFromClass` "/Game/Blueprint/Actors/DungeonFloor.DungeonFloor_C" (`KismetMathLibrary.MakeTransform` (`KismetMathLibrary.MakeVector` (* (- (`KismetMathLibrary.Conv_IntToDouble` _index_2) (/ (`self.XPlane`) 2)) 100.0) (* (- _index (/ (`self.Yplanes`) 2)) 100.0))) "Undefined" "MultiplyWithRoot" null null))
      (if (<= (`KismetMathLibrary.RandomInteger` 100) (`self.ChangedMaxPerct`))
        (`PrimitiveComponent.SetMaterial` (`/Game/Blueprint/Actors/DungeonFloor.Plane` _returnvalue) 0 (`KismetArrayLibrary.Array_Random` (`self.FloorMaterial`)))))))

(fn `UserConstructionScript`)