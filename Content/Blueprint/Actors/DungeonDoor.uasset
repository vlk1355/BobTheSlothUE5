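; Dungeon door actor that swings open and closed by yawing its root component a quarter turn from the starting rotation recorded at BeginPlay.
; The Opendoor event uses a FlipFlop to alternate playing a timeline forward and in reverse, with its track driving the yaw interpolation.
; A CanInteract flag blocks new triggers during movement, and the timeline's finish re-enables it and toggles IsOpen.
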(event `self.ReceiveBeginPlay`
  (bind (_relativerotation_roll _relativerotation_pitch _relativerotation_yaw) (`KismetMathLibrary.BreakRotator` (`SceneComponent.RelativeRotation` (`self.DefaultSceneRoot`))))
  (set `self.RotationStart` _relativerotation_yaw))

(event `Open door`
  (bind _rotationstart (`self.RotationStart`))
  (if (`self.CanInteract`)
    (`/Engine/EditorBlueprintResources/StandardMacros.FlipFlop`
      (:`A`
        (set `self.CanInteract` false)
        (bind (_direction _opentrack) (`Timeline|OpenDoorTimeline` :!via `PlayFromStart` :!label _label)
          (:`Update`
            (`SceneComponent.K2_SetRelativeRotation` (`self.DefaultSceneRoot`) (`KismetMathLibrary.MakeRotator` 0.0 0.0 (`KismetMathLibrary.Lerp` _rotationstart (+ _rotationstart 90.0) _opentrack)) false false))
          (:`Finished`
            (set `self.CanInteract` true)
            (set `self.IsOpen` (not (`self.IsOpen`))))))
      (:`B`
        (set `self.CanInteract` false)
        (goto _label :!via `ReverseFromEnd`)))))

(fn `UserConstructionScript`)